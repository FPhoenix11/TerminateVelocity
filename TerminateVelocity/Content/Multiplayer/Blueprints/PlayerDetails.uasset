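; PlayerDetails is the multiplayer game instance that runs sessions, the lobby, travel and match end.
; UI events create, find and join advanced sessions, filling server lists and opening LobbyMenu as a listen server.
; It builds a player array from names and saved colours, pushes it to controllers, and enables Start when non-host players are ready.
; Start server-travels to ThirdPersonMap; recorded deaths trigger VictoryMap when one player remains.
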(event `LoadPlayerData`
  (`KismetSystemLibrary.PrintString` "Load Pass"))

(event `UpdateLobbyGameState`
  (for (_ _array_index) (`GameStateBase.PlayerArray` (`GameplayStatics.GetGameState`))
    (bind _asblu_player_controller (cast `/Game/ThirdPerson/Blueprints/blu_player_controller` (`GameplayStatics.GetPlayerController` _array_index)))
    (`/Game/ThirdPerson/Blueprints/blu_player_controller.UpdateLobbyState` _asblu_player_controller (`self.PlayerArray`) (`self.PlayerColourArray`))))

(event `UICreateSession`
  (params (VarLAN :type Boolean))
  (`CreateSessionCallbackProxyAdvanced.CreateAdvancedSession` :`PlayerController` (`GameplayStatics.GetPlayerController` 0) :`PublicConnections` (`self.PublicConnections`) :`bUseLAN` VarLAN
    (:`OnSuccess`
      (bind _asplayer_details (cast `/Game/Multiplayer/Blueprints/PlayerDetails` (`GameplayStatics.GetGameInstance`)))
      (set `/Game/Multiplayer/Blueprints/PlayerDetails.PlayerName` "" _asplayer_details)
      (`GameplayStatics.OpenLevel` "LobbyMenu" true "listen"))
    (:`OnFailure`
      (`KismetSystemLibrary.PrintString` "Failure"))))

(event `UIFindSession`
  (params (VarScrollBox :type "PanelWidget Object Reference") (VarFindSessionButton :type "PanelWidget Object Reference") (VarLAN :type Boolean))
  (bind _returnvalue (`GameplayStatics.GetPlayerController` 0))
  (bind _wbcreatesessionmenu (`self.WBCreateSessionMenu`))
  (`PanelWidget.ClearChildren` VarScrollBox)
  (`Widget.SetIsEnabled` VarFindSessionButton false)
  (bind _results (`FindSessionsCallbackProxyAdvanced.FindSessionsAdvanced` _returnvalue 25 VarLAN "AllServers")
    (:`OnSuccess`
      (`KismetSystemLibrary.PrintString` "Search Success")
      (`KismetSystemLibrary.PrintString` (`KismetStringLibrary.Conv_IntToString` (`KismetArrayLibrary.Array_Length` _results)))
      (for _array_element _results
        (bind _returnvalue_2 (`|CreateWidget` "/Game/Multiplayer/Widgets/WB_JoinSession.WB_JoinSession_C" _returnvalue _array_element "" (`/Game/Multiplayer/Widgets/WB_CreateSession.Linear Color Main` _wbcreatesessionmenu) (`/Game/Multiplayer/Widgets/WB_CreateSession.Linear Color Secondary` _wbcreatesessionmenu)))
        (`PanelWidget.AddChild` VarScrollBox _returnvalue_2)
        (`PanelWidget.AddChild` VarScrollBox _returnvalue_2)
        (`PanelWidget.AddChild` VarScrollBox _returnvalue_2)
        (`/Game/Multiplayer/Widgets/WB_JoinSession.WBUpdateServerInfo` _returnvalue_2 _array_element)))
    (:`OnFailure`
      (`KismetSystemLibrary.PrintString` "Search Failed")))
  (`Widget.SetIsEnabled` VarFindSessionButton true))

(event `UILobbySetPlayEnable`
  (set `self.TempCondition` true)
  (for (_array_element _array_index) (`GameStateBase.PlayerArray` (`GameplayStatics.GetGameState`))
    (if (not (== _array_index 0))
      (bind _asblu_player_controller (cast `/Game/ThirdPerson/Blueprints/blu_player_controller` (`PlayerState.GetPlayerController` _array_element)))
      (if (not (`/Game/ThirdPerson/Blueprints/blu_player_controller.PlayerReady` _asblu_player_controller))
        (set `self.TempCondition` false))))
  (bind _foundwidgets (`WidgetBlueprintLibrary.GetAllWidgetsOfClass` "/Game/Multiplayer/Widgets/WB_LobbyMenu.WB_LobbyMenu_C"))
  (`Widget.SetIsEnabled` (`/Game/Multiplayer/Widgets/WB_LobbyMenu.ButtonStart` (`|GetArrayItem` _foundwidgets)) (`self.TempCondition`)))

(event `UIGoToLevel`
  (`KismetSystemLibrary.ExecuteConsoleCommand` (`KismetStringLibrary.Concat_StrStr` "servertravel " "ThirdPersonMap") null)
  (bind _foundwidgets (`WidgetBlueprintLibrary.GetAllWidgetsOfClass` "/Script/UMG.UserWidget" false))
  (for _array_element _foundwidgets
    (if (not (== _array_element "/Game/UI/UICursor.UICursor"))
      (`Widget.RemoveFromParent` _array_element)
      (bind _returnvalue (`|CreateWidget` "/Game/Multiplayer/Widgets/UILoading.UILoading_C" (`GameplayStatics.GetPlayerController` 0)))
      (`UserWidget.AddToViewport` _returnvalue 0))))

(event `UIJoinSession`
  (params (VarSearchResult :type "BlueprintSessionResult Structure"))
  (`JoinSessionCallbackProxy.JoinSession` (`GameplayStatics.GetPlayerController` 0) VarSearchResult
    (:`OnSuccess`
      (`KismetSystemLibrary.PrintString` "True"))
    (:`OnFailure`
      (`KismetSystemLibrary.PrintString` "False"))))

(event `UIGetSessionDetails`
  (params (VarSearchResult :type "BlueprintSessionResult Structure") (VarServerName :type "TextBlock Object Reference") (VarPlayers :type "TextBlock Object Reference") (VarPing :type "TextBlock Object Reference"))
  (`TextBlock.SetText` VarServerName (`KismetTextLibrary.Conv_StringToText` (`FindSessionsCallbackProxy.GetServerName` VarSearchResult)))
  (`TextBlock.SetText` VarPlayers (`KismetTextLibrary.Conv_StringToText` (`KismetStringLibrary.Concat_StrStr` (`KismetStringLibrary.Conv_IntToString` (`FindSessionsCallbackProxy.GetCurrentPlayers` VarSearchResult)) "/" (`KismetStringLibrary.Conv_IntToString` (`FindSessionsCallbackProxy.GetMaxPlayers` VarSearchResult)))))
  (`TextBlock.SetText` VarPing (`KismetTextLibrary.Conv_IntToText` (`FindSessionsCallbackProxy.GetPingInMs` VarSearchResult))))

(event `DeathChecker`
  (`self.DeathCheckerMulti`))

(event `UIRefreshLobbyPlayers`
  (`self.UIRefreshLobbyPlayersMulti` (`self.PlayerArray`)))

(event `DeathCheckerMulti`
  (if (== (`KismetArrayLibrary.Array_Length` (`self.DeathArray`)) (- (`KismetArrayLibrary.Array_Length` (`self.PlayerArray`)) 1))
    (`KismetSystemLibrary.ExecuteConsoleCommand` (`KismetStringLibrary.Concat_StrStr` "servertravel " "VictoryMap") (`GameplayStatics.GetPlayerController` 0))))

(event `UIRefreshLobbyPlayersMulti`
  (params (VarPlayerArray :type "Array of /Game/Multiplayer/PlayerStructure Structure"))
  (bind _asblu_player_controller (cast `/Game/ThirdPerson/Blueprints/blu_player_controller` (`GameplayStatics.GetPlayerController` 0)))
  (`PanelWidget.ClearChildren` (`/Game/Multiplayer/Widgets/WB_LobbyMenu.SessionList_Scrollbx` (`/Game/ThirdPerson/Blueprints/blu_player_controller.WBLobby Menu` _asblu_player_controller)))
  (for _array_element VarPlayerArray
    (`KismetSystemLibrary.PrintString` (`.Name_2_8F798C114B65C2D6238214A93C7EE505` (break `/Game/Multiplayer/PlayerStructure` _array_element))))
  (for _array_element_2 VarPlayerArray
    (bind _returnvalue (`|CreateWidget` "/Game/Multiplayer/Widgets/WB_PlayerInfo.WB_PlayerInfo_C" null (`.Name_2_8F798C114B65C2D6238214A93C7EE505` (break `/Game/Multiplayer/PlayerStructure` _array_element_2))))
    (`PanelWidget.AddChild` (`/Game/Multiplayer/Widgets/WB_LobbyMenu.SessionList_Scrollbx` (`/Game/ThirdPerson/Blueprints/blu_player_controller.WBLobby Menu` _asblu_player_controller)) _returnvalue)))

(event `DeathAdder`
  (params (`Player Num` :type Integer))
  (bind _aslobby_player_state (cast `/Game/Multiplayer/LobbyPlayerState` (`GameplayStatics.GetPlayerState` `Player Num`)))
  (`KismetArrayLibrary.Array_Add` (`self.DeathArray`) (`|GetArrayItem` (`/Game/Multiplayer/LobbyPlayerState.PlayerStructureArray` _aslobby_player_state) `Player Num`))
  (`self.DeathChecker`))

(event `AddPlayerToArray`
  (bind _output (`|GetArrayItem` (`GameStateBase.PlayerArray` (`GameplayStatics.GetGameState`)) (`self.PlayerNumber`)))
  (cast `/Game/Multiplayer/LobbyPlayerState` _output)
  (bind _returnvalue (`GameplayStatics.LoadGameFromSlot` "multiSave"))
  (bind _assave_file (cast `/Game/Multiplayer/SaveFile` _returnvalue))
  (`KismetArrayLibrary.Array_Add` (`self.PlayerArray`) (make `/Game/Multiplayer/PlayerStructure` (`PlayerState.GetPlayerName` _output) (`/Game/Multiplayer/SaveFile.PlayerMainColour` _assave_file) (`/Game/Multiplayer/SaveFile.PlayerSecondaryColour` _assave_file))))

(event `UpdatePlayerStateArray`
  (for _ (`GameStateBase.PlayerArray` (`GameplayStatics.GetGameState`))
    _))

(event `IncrementPlayerNumber`
  (bind _result (`/Engine/EditorBlueprintResources/StandardMacros.IncrementInt` (`self.PlayerNumber`))
    (:`  `
      (set `self.PlayerNumber` _result))))

(fn `OnRep_PlayerArray`)

(fn `UISetPublicConnections`
  (params (PublicConnectionInput :type "Float (double-precision)"))
  (set `self.PublicConnections` (`KismetMathLibrary.FTrunc` PublicConnectionInput))
  (return))

(fn `UISetServerDetails`
  (params (VarServerName :type "TextBlock Object Reference") (VarPlayers :type "TextBlock Object Reference") (VarPing :type "TextBlock Object Reference") (VarSessionResult :type "BlueprintSessionResult Structure")))

(fn `UIShow Lobby Menu`
  (bind _returnvalue (`GameplayStatics.GetPlayerController` 0))
  (`/Engine/EditorBlueprintResources/StandardMacros.IsValid` (`self.WBLobbyMenu`)
    (:`Is Valid`
      _)
    (:`Is Not Valid`
      (bind _returnvalue_2 (`|CreateWidget` "/Game/Multiplayer/Widgets/WB_LobbyMenu.WB_LobbyMenu_C" _returnvalue))
      (set `self.WBLobbyMenu` _returnvalue_2)))
  (`UserWidget.AddToViewport` (`self.WBLobbyMenu`) 0)
  (set `PlayerController.bShowMouseCursor` true _returnvalue)
  (`KismetSystemLibrary.PrintString` "Lobby Menu Generated")
  (return))

(fn `UIShow Multiplayer Menu`
  (bind _returnvalue (`GameplayStatics.GetPlayerController` 0))
  (`/Engine/EditorBlueprintResources/StandardMacros.IsValid` (`self.WBCreateSessionMenu`)
    (:`Is Valid`
      _)
    (:`Is Not Valid`
      (bind _returnvalue_2 (`|CreateWidget` "/Game/Multiplayer/Widgets/WB_CreateSession.WB_CreateSession_C" _returnvalue))
      (set `self.WBCreateSessionMenu` _returnvalue_2)))
  (`UserWidget.AddToViewport` (`self.WBCreateSessionMenu`) 0)
  (`WidgetBlueprintLibrary.SetInputMode_UIOnlyEx` _returnvalue null)
  (set `PlayerController.bShowMouseCursor` true _returnvalue)
  (return))